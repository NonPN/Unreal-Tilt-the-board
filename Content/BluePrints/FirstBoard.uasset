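; FirstBoard is an actor Blueprint that lets the player tilt a Board component with the mouse.
; MouseX axis input adds to the Board's world roll, and MouseY adds to its pitch, leaving yaw unchanged.
; Each change is applied directly to world rotation by the raw axis value, with no clamping or delta-time scaling.
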(event `InputAxisKey|MouseX`
  (params (AxisValue :type "Float (single-precision)"))
  (bind _board (`self.Board`))
  (`SceneComponent.K2_SetWorldRotation` _board (`KismetMathLibrary.MakeRotator` (+ (.roll (`SceneComponent.K2_GetComponentRotation` _board)) AxisValue) (.pitch (`SceneComponent.K2_GetComponentRotation` _board)) (.yaw (`SceneComponent.K2_GetComponentRotation` _board))) false false))

(event `InputAxisKey|MouseY`
  (params (AxisValue :type "Float (single-precision)"))
  (bind _board (`self.Board`))
  (`SceneComponent.K2_SetWorldRotation` _board (`KismetMathLibrary.MakeRotator` (.roll (`SceneComponent.K2_GetComponentRotation` _board)) (+ (.pitch (`SceneComponent.K2_GetComponentRotation` _board)) AxisValue) (.yaw (`SceneComponent.K2_GetComponentRotation` _board))) false false))

(fn `UserConstructionScript`)