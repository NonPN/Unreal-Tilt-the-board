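; Level board actor for a tilt-the-board ball game: it spawns a Ball and rotates its mesh with mouse X/Y.
; A Delay-gated Tick cycles the Taser material across six cubes, and hitting the active one triggers slow motion, destroys ball and board, and shows GameOver.
; Hitting Goal2 arms Goal1, which then shows the Goal widget.
; Pause and both endings flag the InGame widget as ended.
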(event `InputAction|Pause`
  (params (Key :type "Key Structure"))
  (:`Pressed`
    (if (not (`self.gameEnd`))
      (bind _asin_game (castclass `/Game/Widgets/InGame` "/Game/Widgets/InGame.InGame_C"))
      (bind _foundwidgets (`WidgetBlueprintLibrary.GetAllWidgetsOfClass` _asin_game))
      (set `/Game/Widgets/InGame.isGameEnd` true (`|GetArrayItem` _foundwidgets))
      (`GameplayStatics.SetGamePaused` true)
      (bind _returnvalue (`|CreateWidget` "/Game/Widgets/Pause.Pause_C" (`GameplayStatics.GetPlayerController` 0)))
      (`UserWidget.AddToViewport` _returnvalue 0))))

(event `self.ReceiveBeginPlay`
  (set `self.gameEnd` false)
  (set `self.firstHit` true)
  (set `self.goal2Entered` false)
  (bind _returnvalue (`|SpawnActorFromClass` "/Game/BluePrints/ball.ball_C" (`SceneComponent.K2_GetComponentToWorld` (`self.spawn_point`)) "Undefined" "OverrideRootScale" null null))
  (set `self.Ball` _returnvalue))

(event `InputAxisKey|MouseX`
  (params (AxisValue :type "Float (single-precision)"))
  (bind _staticmesh (`self.StaticMesh`))
  ;[1 1 1] Tilt the board
  (`SceneComponent.K2_SetWorldRotation` _staticmesh (`KismetMathLibrary.MakeRotator` (.roll (`SceneComponent.K2_GetComponentRotation` _staticmesh)) (+ (.pitch (`SceneComponent.K2_GetComponentRotation` _staticmesh)) AxisValue) (.yaw (`SceneComponent.K2_GetComponentRotation` _staticmesh))) false false))

(event `InputAxisKey|MouseY`
  (params (AxisValue :type "Float (single-precision)"))
  (bind _staticmesh (`self.StaticMesh`))
  ;[1 1 1] Tilt the board
  (`SceneComponent.K2_SetWorldRotation` _staticmesh (`KismetMathLibrary.MakeRotator` (+ (.roll (`SceneComponent.K2_GetComponentRotation` _staticmesh)) AxisValue) (.pitch (`SceneComponent.K2_GetComponentRotation` _staticmesh)) (.yaw (`SceneComponent.K2_GetComponentRotation` _staticmesh))) false false))

(event `self.ReceiveTick`
  (params (DeltaSeconds :type "Float (single-precision)"))
  (bind _cube2 (`self.cube2`))
  (bind _cube3 (`self.cube3`))
  (bind _cube4 (`self.cube4`))
  (bind _cube5 (`self.cube5`))
  (bind _cube6 (`self.cube6`))
  (bind _cube_num (`self.cube_num`))
  (bind _cube6_2 (`self.cube6`))
  (bind _cube1 (`self.cube1`))
  (bind _cube2_2 (`self.cube2`))
  (bind _cube3_2 (`self.cube3`))
  (bind _cube4_2 (`self.cube4`))
  (bind _cube5_2 (`self.cube5`))
  (bind _cube1_2 (`self.cube1`))
  (`KismetSystemLibrary.Delay` 1.0)
  (if (== _cube_num 0)
    (`PrimitiveComponent.SetMaterialByName` _cube6_2 (`|GetArrayItem` (`MeshComponent.GetMaterialSlotNames` _cube6_2)) "/Game/StarterContent/Materials/M_Basic_Floor.M_Basic_Floor")
    (else
      (switch `int` (- _cube_num 1)
        (:`0`
          (`PrimitiveComponent.SetMaterialByName` _cube1 (`|GetArrayItem` (`MeshComponent.GetMaterialSlotNames` _cube1)) "/Game/StarterContent/Materials/M_Basic_Floor.M_Basic_Floor"))
        (:`1`
          (`PrimitiveComponent.SetMaterialByName` _cube2_2 (`|GetArrayItem` (`MeshComponent.GetMaterialSlotNames` _cube2_2)) "/Game/StarterContent/Materials/M_Basic_Floor.M_Basic_Floor"))
        (:`2`
          (`PrimitiveComponent.SetMaterialByName` _cube3_2 (`|GetArrayItem` (`MeshComponent.GetMaterialSlotNames` _cube3_2)) "/Game/StarterContent/Materials/M_Basic_Floor.M_Basic_Floor"))
        (:`3`
          (`PrimitiveComponent.SetMaterialByName` _cube4_2 (`|GetArrayItem` (`MeshComponent.GetMaterialSlotNames` _cube4_2)) "/Game/StarterContent/Materials/M_Basic_Floor.M_Basic_Floor"))
        (:`4`
          (`PrimitiveComponent.SetMaterialByName` _cube5_2 (`|GetArrayItem` (`MeshComponent.GetMaterialSlotNames` _cube5_2)) "/Game/StarterContent/Materials/M_Basic_Floor.M_Basic_Floor")))))
  (switch `int` (`self.cube_num`)
    (:`Default`
      (`PrimitiveComponent.SetMaterialByName` _cube1_2 (`|GetArrayItem` (`MeshComponent.GetMaterialSlotNames` _cube1_2)) "/Game/Materials/taser_Inst.taser_Inst" :!label _label)
      (if (== (`self.cube_num`) 5)
        (set `self.cube_num` 0)
        (else
          (set `self.cube_num` (+ (`self.cube_num`) 1))))
      (`KismetSystemLibrary.Delay` 1.0))
    (:`0`
      (goto _label))
    (:`1`
      (`PrimitiveComponent.SetMaterialByName` _cube2 (`|GetArrayItem` (`MeshComponent.GetMaterialSlotNames` _cube2)) "/Game/Materials/taser_Inst.taser_Inst")
      (if (== (`self.cube_num`) 5)
        (set `self.cube_num` 0)
        (else
          (set `self.cube_num` (+ (`self.cube_num`) 1))))
      (`KismetSystemLibrary.Delay` 1.0))
    (:`2`
      (`PrimitiveComponent.SetMaterialByName` _cube3 (`|GetArrayItem` (`MeshComponent.GetMaterialSlotNames` _cube3)) "/Game/Materials/taser_Inst.taser_Inst")
      (if (== (`self.cube_num`) 5)
        (set `self.cube_num` 0)
        (else
          (set `self.cube_num` (+ (`self.cube_num`) 1))))
      (`KismetSystemLibrary.Delay` 1.0))
    (:`3`
      (`PrimitiveComponent.SetMaterialByName` _cube4 (`|GetArrayItem` (`MeshComponent.GetMaterialSlotNames` _cube4)) "/Game/Materials/taser_Inst.taser_Inst")
      (if (== (`self.cube_num`) 5)
        (set `self.cube_num` 0)
        (else
          (set `self.cube_num` (+ (`self.cube_num`) 1))))
      (`KismetSystemLibrary.Delay` 1.0))
    (:`4`
      (`PrimitiveComponent.SetMaterialByName` _cube5 (`|GetArrayItem` (`MeshComponent.GetMaterialSlotNames` _cube5)) "/Game/Materials/taser_Inst.taser_Inst")
      (if (== (`self.cube_num`) 5)
        (set `self.cube_num` 0)
        (else
          (set `self.cube_num` (+ (`self.cube_num`) 1))))
      (`KismetSystemLibrary.Delay` 1.0))
    (:`5`
      (`PrimitiveComponent.SetMaterialByName` _cube6 (`|GetArrayItem` (`MeshComponent.GetMaterialSlotNames` _cube6)) "/Game/Materials/taser_Inst.taser_Inst")
      (if (== (`self.cube_num`) 5)
        (set `self.cube_num` 0)
        (else
          (set `self.cube_num` (+ (`self.cube_num`) 1))))
      (`KismetSystemLibrary.Delay` 2.0))))

(event `self.goal1.OnComponentHit`
  (params (HitComponent :type "PrimitiveComponent Object Reference") (OtherActor :type "Actor Object Reference") (OtherComp :type "PrimitiveComponent Object Reference") (NormalImpulse :type "Vector Structure") (Hit :type "HitResult Structure (by ref)"))
  (bind _returnvalue (`GameplayStatics.GetPlayerController` 0))
  (bind _goal1 (`self.goal1`))
  ;[1 1 1] User Enter Goal Tricker
  (if (and (`self.goal2Entered`) (not (`self.gameEnd`)))
    (`GameplayStatics.PlaySound2D` "/Game/Assets/tink.tink" 1.0 1.0 0.0 null null)
    (if (`self.firstHit`)
      (`PrimitiveComponent.SetMaterialByName` _goal1 (`|GetArrayItem` (`MeshComponent.GetMaterialSlotNames` _goal1)) "/Game/Materials/taser_Inst.taser_Inst")
      (set `self.firstHit` false)
      (bind _asin_game (castclass `/Game/Widgets/InGame` "/Game/Widgets/InGame.InGame_C"))
      (bind _foundwidgets (`WidgetBlueprintLibrary.GetAllWidgetsOfClass` _asin_game))
      (bind _output (`|GetArrayItem` _foundwidgets))
      (set `/Game/Widgets/InGame.isGameEnd` true _output)
      (set `self.gameEnd` true)
      (bind _returnvalue_2 (`|CreateWidget` "/Game/Widgets/Goal.Goal_C" _returnvalue))
      (`UserWidget.AddToViewport` _returnvalue_2 0)
      (set `PlayerController.bShowMouseCursor` true _returnvalue)
      (`self.K2_DestroyActor` self)
      (`self.K2_DestroyActor` (`self.Ball`))
      (`/Game/Widgets/InGame.Reset` _output))))

(event `self.cube1.OnComponentHit`
  (params (HitComponent :type "PrimitiveComponent Object Reference") (OtherActor :type "Actor Object Reference") (OtherComp :type "PrimitiveComponent Object Reference") (NormalImpulse :type "Vector Structure") (Hit :type "HitResult Structure (by ref)"))
  (if (== (`self.cube_num`) 1)
    (if (not (`self.gameEnd`)) :!label _label_2
      (`/Engine/EditorBlueprintResources/StandardMacros.DoOnce` false
        (:`Completed`
          (`GameplayStatics.PlaySound2D` "/Game/Assets/loose_impact.loose_impact" 1.0 1.0 0.0 null null)
          (`GameplayStatics.SetGlobalTimeDilation` 0.13)
          (`KismetSystemLibrary.Delay` 0.3)
          (`self.destroy`)
          (bind _asin_game (castclass `/Game/Widgets/InGame` "/Game/Widgets/InGame.InGame_C"))
          (bind _foundwidgets (`WidgetBlueprintLibrary.GetAllWidgetsOfClass` _asin_game))
          (bind _output (`|GetArrayItem` _foundwidgets))
          (set `/Game/Widgets/InGame.isGameEnd` true _output)
          (`/Game/Widgets/InGame.Reset` _output)
          (set `self.gameEnd` true)
          (bind _returnvalue (`|CreateWidget` "/Game/Widgets/GameOVer.GameOver_C" (`GameplayStatics.GetPlayerController` 0)))
          (`UserWidget.AddToViewport` _returnvalue 0))))))

(event `self.cube2.OnComponentHit`
  (params (HitComponent :type "PrimitiveComponent Object Reference") (OtherActor :type "Actor Object Reference") (OtherComp :type "PrimitiveComponent Object Reference") (NormalImpulse :type "Vector Structure") (Hit :type "HitResult Structure (by ref)"))
  (if (== (`self.cube_num`) 2)
    (goto _label_2)))

(event `self.cube3.OnComponentHit`
  (params (HitComponent :type "PrimitiveComponent Object Reference") (OtherActor :type "Actor Object Reference") (OtherComp :type "PrimitiveComponent Object Reference") (NormalImpulse :type "Vector Structure") (Hit :type "HitResult Structure (by ref)"))
  (if (== (`self.cube_num`) 3)
    (goto _label_2)))

(event `self.cube4.OnComponentHit`
  (params (HitComponent :type "PrimitiveComponent Object Reference") (OtherActor :type "Actor Object Reference") (OtherComp :type "PrimitiveComponent Object Reference") (NormalImpulse :type "Vector Structure") (Hit :type "HitResult Structure (by ref)"))
  (if (== (`self.cube_num`) 4)
    (goto _label_2)))

(event `self.cube5.OnComponentHit`
  (params (HitComponent :type "PrimitiveComponent Object Reference") (OtherActor :type "Actor Object Reference") (OtherComp :type "PrimitiveComponent Object Reference") (NormalImpulse :type "Vector Structure") (Hit :type "HitResult Structure (by ref)"))
  (if (== (`self.cube_num`) 5)
    (goto _label_2)))

(event `self.cube6.OnComponentHit`
  (params (HitComponent :type "PrimitiveComponent Object Reference") (OtherActor :type "Actor Object Reference") (OtherComp :type "PrimitiveComponent Object Reference") (NormalImpulse :type "Vector Structure") (Hit :type "HitResult Structure (by ref)"))
  (if (== (`self.cube_num`) 0)
    (goto _label_2)))

(event `self.goal2.OnComponentHit`
  (params (HitComponent :type "PrimitiveComponent Object Reference") (OtherActor :type "Actor Object Reference") (OtherComp :type "PrimitiveComponent Object Reference") (NormalImpulse :type "Vector Structure") (Hit :type "HitResult Structure (by ref)"))
  (bind _goal2 (`self.goal2`))
  ;[1 1 1] Goal2 entered
  (if (not (`self.goal2Entered`))
    (`GameplayStatics.PlaySound2D` "/Game/Assets/tink.tink" 1.0 1.0 0.0 null null)
    (`PrimitiveComponent.SetMaterialByName` _goal2 (`|GetArrayItem` (`MeshComponent.GetMaterialSlotNames` _goal2)) "/Game/Materials/taser_Inst.taser_Inst")
    (set `self.goal2Entered` true)))

(fn `destroy`
  (`self.K2_DestroyActor` (`self.Ball`))
  (`self.K2_DestroyActor` self))

(fn `UserConstructionScript`)