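; Board actor for a tilt-the-board ball game that spawns a ball at its spawn point on BeginPlay.
; Mouse X and Y axes add pitch and roll to the board mesh to tilt it.
; The first hit on the Goal component plays a sound, swaps its material, flags the InGame widget as ended and shows a goal screen.
; It then destroys the ball and itself and resets the InGame widget.
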(event `self.ReceiveBeginPlay`
  (bind _returnvalue (`|SpawnActorFromClass` "/Game/BluePrints/ball.ball_C" (`SceneComponent.K2_GetComponentToWorld` (`self.spawn_point`)) "Undefined" "OverrideRootScale" null null))
  (set `self.Ball` _returnvalue))

(event `InputAxisKey|MouseX`
  (params (AxisValue :type "Float (single-precision)"))
  (bind _staticmesh (`self.StaticMesh`))
  ;[1 1 1] Tilt the board
  (`SceneComponent.K2_SetWorldRotation` _staticmesh (`KismetMathLibrary.MakeRotator` (.roll (`SceneComponent.K2_GetComponentRotation` _staticmesh)) (+ (.pitch (`SceneComponent.K2_GetComponentRotation` _staticmesh)) AxisValue) (.yaw (`SceneComponent.K2_GetComponentRotation` _staticmesh))) false false))

(event `InputAxisKey|MouseY`
  (params (AxisValue :type "Float (single-precision)"))
  (bind _staticmesh (`self.StaticMesh`))
  ;[1 1 1] Tilt the board
  (`SceneComponent.K2_SetWorldRotation` _staticmesh (`KismetMathLibrary.MakeRotator` (+ (.roll (`SceneComponent.K2_GetComponentRotation` _staticmesh)) AxisValue) (.pitch (`SceneComponent.K2_GetComponentRotation` _staticmesh)) (.yaw (`SceneComponent.K2_GetComponentRotation` _staticmesh))) false false))

(event `self.goal.OnComponentHit`
  (params (HitComponent :type "PrimitiveComponent Object Reference") (OtherActor :type "Actor Object Reference") (OtherComp :type "PrimitiveComponent Object Reference") (NormalImpulse :type "Vector Structure") (Hit :type "HitResult Structure (by ref)"))
  (bind _returnvalue (`GameplayStatics.GetPlayerController` 0))
  (bind _goal (`self.goal`))
  ;[1 1 1] User Enter Goal Tricker
  (if (not (`self.gameEnd`))
    (set `self.gameEnd` true)
    (`GameplayStatics.PlaySound2D` "/Game/Assets/tink.tink" 1.0 1.0 0.0 null null)
    (`PrimitiveComponent.SetMaterialByName` _goal (`|GetArrayItem` (`MeshComponent.GetMaterialSlotNames` _goal)) "/Game/Materials/taser_Inst.taser_Inst")
    (bind _asin_game (castclass `/Game/Widgets/InGame` "/Game/Widgets/InGame.InGame_C"))
    (bind _foundwidgets (`WidgetBlueprintLibrary.GetAllWidgetsOfClass` _asin_game))
    (bind _output (`|GetArrayItem` _foundwidgets))
    (set `/Game/Widgets/InGame.isGameEnd` true _output)
    (bind _returnvalue_2 (`|CreateWidget` "/Game/Widgets/Goal.Goal_C" _returnvalue))
    (`UserWidget.AddToViewport` _returnvalue_2 0)
    (set `PlayerController.bShowMouseCursor` true _returnvalue)
    (`WidgetBlueprintLibrary.SetFocusToGameViewport`)
    (`self.K2_DestroyActor` (`self.Ball`))
    (`self.K2_DestroyActor` self)
    (`/Game/Widgets/InGame.Reset` _output)))

(fn `UserConstructionScript`)